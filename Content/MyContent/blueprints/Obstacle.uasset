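; Obstacle actor that uses physics impulses to home in on the player pawn.
; While IsHoming is set, each Tick applies an impulse to its Sphere, computed by ImpulseToPlayer from the obstacle and player locations.
; Any actor overlap starts a one-second timer that calls StopHoming, which clears the flag and ends the pursuit.
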(event EventBeginPlay)

(event Collision|EventActorBeginOverlap
  (params (OtherActor :type Actor%20Object%20Reference))
  (Utilities|Time|SetTimerbyFunctionName 0 "StopHoming" 1.0))

(event EventTick
  (params (DeltaSeconds :type Float%20%28single-precision%29))
  (if (Variables|Default|GetIsHoming)
    (Physics|AddImpulse (Variables|Default|GetSphere) (Class|ProjectileMovementBPLibrary|ImpulsetoPlayer 1e+05 (Transformation|GetActorLocation) (Transformation|GetActorLocation (Game|Player|GetPlayerPawn 0))) "None" false)))

(fn ConstructionScript)

(fn StopHoming
  (Variables|Default|SetIsHoming false))