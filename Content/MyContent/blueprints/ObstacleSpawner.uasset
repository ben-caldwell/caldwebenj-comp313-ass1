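; ObstacleSpawner is an actor that repeatedly spawns Obstacle actors at its own location and launches them upward.
; SpawnObstacle runs on BeginPlay, spawns an Obstacle with zero rotation, and applies a large Z impulse to its Sphere component.
; It then re-arms itself by function-name timer with a random delay of one to four seconds, but only if the spawn succeeded, so a failed spawn ends the loop.
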(event EventBeginPlay
  (CallFunction|SpawnObstacle))

(event Collision|EventActorBeginOverlap
  (params (OtherActor :type Actor%20Object%20Reference)))

(event EventTick
  (params (DeltaSeconds :type Float%20%28single-precision%29)))

(fn ConstructionScript)

(fn SpawnObstacle
  (bind _returnvalue (Game|SpawnActorfromClass "/Game/MyContent/blueprints/Obstacle.Obstacle_C" (Math|Transform|MakeTransform (.Location (Math|Transform|BreakTransform (Transformation|GetActorTransform)))) "Undefined" 0 0))
  (if (Utilities|IsValid _returnvalue)
    (Physics|AddImpulse (Variables|/Game/MyContent/blueprints/Obstacle.Obstacle_C|GetSphere _returnvalue) "0, 0,1700000.000000" "None" false)
    (Utilities|Time|SetTimerbyFunctionName 0 "SpawnObstacle" (+ (* (Math|Random|RandomFloat) 3.0) 1.0))))