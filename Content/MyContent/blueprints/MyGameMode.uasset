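; MyGameMode is a game mode Blueprint that tracks the score and elapsed time of the current run.
; BeginPlay calls Restart, which stores the current game time as StartTime and zeroes Score.
; GetCurrentRunTime derives elapsed time from StartTime on demand, so no Tick logic is used, and AddToScore adds a given value to Score.
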(event EventBeginPlay
  (CallFunction|Restart))

(event EventTick
  (params (DeltaSeconds :type Float%20%28single-precision%29)))

(fn ConstructionScript)

(fn GetCurrentRunTime
  (return (- (Utilities|Time|GetGameTimeinSeconds) (Variables|Default|GetStartTime))))

(fn Restart
  (Variables|Default|SetStartTime (Utilities|Time|GetGameTimeinSeconds))
  (Variables|Default|SetScore 0))

(fn AddtoScore
  (params (AddValue :type Integer))
  (Variables|Default|SetScore (+ AddValue (Variables|Default|GetScore))))