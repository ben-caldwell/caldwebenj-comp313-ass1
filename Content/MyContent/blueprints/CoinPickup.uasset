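; CoinPickup is a collectible coin actor that spins in place and awards score when picked up.
; On BeginPlay, a timeline drives the cylinder mesh's yaw, offset from its initial world rotation.
; Any overlap with the sphere component destroys the actor, adds a fixed amount to the score through MyGameMode and plays a pickup sound at its location.
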(event OnComponentBeginOverlap(Sphere)
  (params (OverlappedComponent :type Primitive%20Component%20Object%20Reference) (OtherActor :type Actor%20Object%20Reference) (OtherComp :type Primitive%20Component%20Object%20Reference) (OtherBodyIndex :type Integer) (bFromSweep :type Boolean) (SweepResult :type Hit%20Result%20Structure%20%28by%20ref%29))
  (Actor|DestroyActor)
  (bind _asmy_game_mode (Utilities|Casting|CastToMyGameMode (Game|GetGameMode)))
  (Default|AddtoScore _asmy_game_mode 10)
  (Audio|PlaySoundatLocation "/Game/MyContent/sounds/snd_coin_pickup.snd_coin_pickup" (Transformation|GetActorLocation) "0, 0, 0" 1.0 1.0 0.0 0 0 0))

(event EventBeginPlay
  ;[1 1 1] Rotate Coin
  (Variables|Default|SetInitialRotation (Transformation|GetWorldRotation (Variables|Default|GetCylinder)))
  (bind _newtrack_0 (Timeline|Timeline_0 Play)
    (:Update
      (Transformation|SetWorldRotation (Variables|Default|GetCylinder) (Math|Rotator|MakeRotator (.roll (Variables|Default|GetInitialRotation)) (.pitch (Variables|Default|GetInitialRotation)) (+ _newtrack_0 (.yaw (Variables|Default|GetInitialRotation)))) false false))))

(event Collision|EventActorBeginOverlap
  (params (OtherActor :type Actor%20Object%20Reference)))

(event EventTick
  (params (DeltaSeconds :type Float%20%28single-precision%29)))

(fn ConstructionScript)